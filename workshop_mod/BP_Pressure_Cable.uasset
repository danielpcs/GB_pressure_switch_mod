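; BP_Pressure_Cable is a firearm attachment that visually connects a PEQ-15 plug to a pressure switch on the same weapon.
; When equipped, it finds the first BP_Pressure_Switch among the parent firearm's attached actors.
; It then stretches a spline mesh from the plug to the switch pad's "Cable" socket, converting both points to cable-local space with fixed tangents, and hides its mount point.
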(event EventBeginPlay)

(event Collision|EventActorBeginOverlap
  (params (OtherActor :type Actor%20Object%20Reference)))

(event EventTick
  (params (DeltaSeconds :type Float%20%28single-precision%29)))

(event EventOnBeingEquipped
  (|CallParentFunction)
  (CallFunction|GenerateCable))

(fn ConstructionScript
  (|CallParentFunction))

(fn GenerateCable
  (bind _cable (Variables|Default|GetCable))
  (bind _returnvalue (Transformation|GetWorldTransform _cable))
  (bind _returnvalue_2 (Class|GBRailAttachment|GetParentFirearm self))
  (bind _asbp_firearm_master (Utilities|Casting|CastToBP_Firearm_Master _returnvalue_2))
  (Utilities|IsValid _asbp_firearm_master
    (:Is%20Valid
      (bind _filteredarray (Utilities|Array|FilterArray (Actor|GetAttachedActors _asbp_firearm_master true) "/SecondTryPressurePad/3327713435/BP_Pressure_Switch.BP_Pressure_Switch_C"))
      (bind _asbp_pressure_switch (Utilities|Casting|CastToBP_Pressure_Switch (Utilities|Array|Get(acopy) _filteredarray)))
      (Utilities|IsValid _asbp_pressure_switch
        (:Is%20Valid
          (SplineMesh|SetStartandEnd _cable (Math|Transform|InverseTransformLocation _returnvalue (Transformation|GetWorldLocation (Variables|Default|Getpressure_pad_peq15_plug))) "0, 0,15.000000" (Math|Transform|InverseTransformLocation _returnvalue (Transformation|GetSocketLocation (Variables|/SecondTryPressurePad/3327713435/BP_Pressure_Switch.BP_Pressure_Switch_C|GetPressurePad _asbp_pressure_switch) "Cable")) "0, 0,15.000000" true :!class /Script/Engine.SplineMeshComponent)
          (Rendering|SetVisibility (Variables|Default|GetMountPoint) false false))))))